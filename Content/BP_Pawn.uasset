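; Player pawn that spawns a BP_Ball at its capsule's transform on BeginPlay, stores it as PlayingBall and takes MoveRight axis input.
; MoveRight feeds the axis value into AddMovementInput along the forward vector of the control rotation with pitch zeroed, despite its name.
; The D key calls MoveRight with zero, and unconnected leftover nodes hold an older sideways world-offset movement.
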(event EventBeginPlay
  (bind _returnvalue (Game|SpawnActorfromClass "/Game/BP_Ball.BP_Ball_C" (Transformation|GetWorldTransform (Variables|Default|GetCapsule)) "AlwaysSpawn" "MultiplyWithRoot" 0 0))
  (Variables|Default|SetPlayingBall _returnvalue))

(event Collision|EventActorBeginOverlap
  (params (OtherActor :type Actor%20Object%20Reference)))

(event EventTick
  (params (DeltaSeconds :type Float%20%28single-precision%29)))

(event Input|AxisEvents|InputAxisMoveRight
  (params (AxisValue :type Float%20%28single-precision%29))
  (CallFunction|MoveRight AxisValue))

(event Input|KeyboardEvents|D
  (params (Key :type Key%20Structure :default "None"))
  (:Pressed
    (CallFunction|MoveRight 0.0)))

(fn ConstructionScript)

(fn MoveRight
  (params (AxisValue :type Float%20%28double-precision%29))
  (bind _returnvalue (Pawn|GetControlRotation :!class /Script/Engine.Pawn))
  (Pawn|Input|AddMovementInput (Math|Vector|GetForwardVector (Math|Rotator|MakeRotator (.roll _returnvalue) 0.0 (.yaw _returnvalue))) AxisValue false))